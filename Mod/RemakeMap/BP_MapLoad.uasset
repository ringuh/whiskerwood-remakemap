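; Mod actor that adds a "Remake map" button above the bottom toolbar on day 1 of a new, non-save game.
; Placement retries on a timer, searching HUD widgets level by level for BottomToolbar_C, then slots the button into its canvas or overlay parent.
; A confirming second click sets a random seed preference and calls EnterPlay to regenerate.
; The button is removed after day 1; a config file enables debug logging.
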(event Custom|OnDayStart
  (params (day :type Integer))
  (if (Variables|Default|GetDebug)
    (Class|ModAPI|LogMessage (Class|ModAPI|GetModAPI) (Utilities|String|Append (Utilities|String|Append (Utilities|String|Append (Utilities|String|Append "RemakeMap: onDayStart day=" "") (Utilities|String|ToString(Integer) day)) " worldTime day=") (Utilities|String|ToString(Integer) (Variables|/Script/ProjectArco.WorldTime|Getm_day (Variables|/Script/ProjectArco.ArcoSystems|Getm_worldTime (Variables|Default|GetArco))))) true))
  (if (and (> day 1) (Utilities|IsValid (Variables|Default|GetButton)))
    (Widget|RemovefromParent (Variables|Default|GetButton))
    (Variables|Default|SetPlaced true)
    (if (Variables|Default|GetDebug)
      (Class|ModAPI|LogMessage (Class|ModAPI|GetModAPI) "RemakeMap: day 1 is over, button removed" true))))

(event Custom|OnLoaded
  (if (not (Variables|Default|GetReady))
    (if (Utilities|IsValid (Game|GetPlayerController 0))
      (Variables|Default|SetReady true)
      (bind _returnvalue (Class|ModAPI|ReadModTextFile (Class|ModAPI|GetModAPI) "RemakeMapConfig" "debug"))
      (Variables|Default|SetDebug (not (Utilities|Array|IsEmpty _returnvalue)))
      (if (Variables|Default|GetDebug)
        (Class|ModAPI|LogMessage (Class|ModAPI|GetModAPI) "RemakeMap ready (v17)" true))
      (bind (_out_isvalid _returnvalue_2) (Class|ArcoSystems|GetArcoSys))
      (Variables|Default|SetArco _returnvalue_2)
      (bind _returnvalue_3 (Class|ArcoSystems|IsSaveGame (Variables|Default|GetArco)))
      (if (Variables|Default|GetDebug)
        (Class|ModAPI|LogMessage (Class|ModAPI|GetModAPI) (Utilities|String|Append (Utilities|String|Append (Utilities|String|Append (Utilities|String|Append (Utilities|String|Append (Utilities|String|Append (Utilities|String|Append (Utilities|String|Append (Utilities|String|Append (Utilities|String|Append "RemakeMap: arco valid=" "") (Utilities|String|ToString(Boolean) _out_isvalid)) " save game=") (Utilities|String|ToString(Boolean) _returnvalue_3)) " day=") (Utilities|String|ToString(Integer) (Variables|/Script/ProjectArco.WorldTime|Getm_day (Variables|/Script/ProjectArco.ArcoSystems|Getm_worldTime (Variables|Default|GetArco))))) " colony=") (Class|ArcoSystems|GetColonyName (Variables|Default|GetArco))) " debt=") (Utilities|String|ToString(Float) (Class|ArcoSystems|GetDebtMultiplier (Variables|Default|GetArco)))) true))
      (if (and (not _returnvalue_3) (<= (Variables|/Script/ProjectArco.WorldTime|Getm_day (Variables|/Script/ProjectArco.ArcoSystems|Getm_worldTime (Variables|Default|GetArco))) 1))
        (bind _returnvalue_4 (UserInterface|CreateWidget "/Game/Mods/RemakeMap/WBP_RemakeButton.WBP_RemakeButton_C" (Game|GetPlayerController 0)))
        (Variables|Default|SetButton _returnvalue_4)
        (Rendering|Components|TextRender|SetText (Variables|/Game/Mods/RemakeMap/WBP_RemakeButton.WBP_RemakeButton_C|GetLabel (Variables|Default|GetButton)) (Utilities|Text|ToText(String) "Remake map"))
        (EventDispatchers|BindEventtoOnClicked (Variables|/Game/Mods/RemakeMap/WBP_RemakeButton.WBP_RemakeButton_C|GetBtn (Variables|Default|GetButton)) (delegate Custom|OnRemakeClick))
        (if (not (or (Variables|Default|GetPlaced) (not (Utilities|IsValid (Variables|Default|GetButton)))))
          (bind _foundwidgets (Widget|GetAllWidgetsOfClass self "/Script/ProjectArco.PlayHud"))
          (if (> (Utilities|Array|Length _foundwidgets) 0)
            (Variables|Default|SetHud 0)
            (for _array_element _foundwidgets
              (Variables|Default|SetHud _array_element))
            (if (Variables|Default|GetDebug)
              (Class|ModAPI|LogMessage (Class|ModAPI|GetModAPI) (Utilities|String|Append (Utilities|String|Append (Utilities|String|Append (Utilities|String|Append "RemakeMap: walking HUD " "") (Utilities|GetDisplayName (Variables|Default|GetHud))) ", try ") (Utilities|String|ToString(Integer) (Variables|Default|GetHudTries))) true))
            (Utilities|Array|Clear (Variables|Default|GetLevel))
            (Utilities|Array|Add (Variables|Default|GetLevel) (Variables|Default|GetHud))
            (Variables|Default|SetTB 0)
            (if (and (not (Utilities|IsValid (Variables|Default|GetTB))) (> (Utilities|Array|Length (Variables|Default|GetLevel)) 0))
              (Utilities|Array|Clear (Variables|Default|GetNext))
              (for _array_element_2 (Variables|Default|GetLevel)
                (if (and (Utilities|Enum|Equal(Enum) (Utilities|GetClassDisplayName (Utilities|GetClass _array_element_2)) "BottomToolbar_C") (not (Utilities|IsValid (Variables|Default|GetTB))))
                  (Variables|Default|SetTB _array_element_2))
                (bind _aspanel_widget (Utilities|Casting|CastToPanelWidget _array_element_2)
                  (:then
                    (Utilities|Array|AppendArray (Variables|Default|GetNext) (Class|PanelWidget|GetAllChildren _aspanel_widget)))
                  (:CastFailed
                    (bind _asuser_widget (Utilities|Casting|CastToUserWidget _array_element_2))
                    (bind _returnvalue_5 (Class|NaviUi|FindDecendentsOfClasses _asuser_widget (Utilities|Array|MakeArray "/Script/UMG.CanvasPanel" "/Script/UMG.Overlay" "/Script/UMG.HorizontalBox" "/Script/UMG.VerticalBox" "/Script/UMG.GridPanel" "/Script/UMG.UniformGridPanel" "/Script/UMG.WrapBox" "/Script/UMG.ScrollBox" "/Script/UMG.SizeBox" "/Script/UMG.Border" "/Script/UMG.ScaleBox" "/Script/UMG.SafeZone" "/Script/UMG.NamedSlot" "/Script/UMG.WidgetSwitcher" "/Script/UMG.InvalidationBox" "/Script/UMG.RetainerBox" "/Script/UMG.StackBox" "/Script/UMG.BackgroundBlur") false))
                    (Utilities|Array|AppendArray (Variables|Default|GetNext) _returnvalue_5))))
              (Variables|Default|SetLevel (Variables|Default|GetNext))
              (if (and (not (Utilities|IsValid (Variables|Default|GetTB))) (> (Utilities|Array|Length (Variables|Default|GetLevel)) 0))
                (Utilities|Array|Clear (Variables|Default|GetNext))
                (for _array_element_3 (Variables|Default|GetLevel)
                  (if (and (Utilities|Enum|Equal(Enum) (Utilities|GetClassDisplayName (Utilities|GetClass _array_element_3)) "BottomToolbar_C") (not (Utilities|IsValid (Variables|Default|GetTB))))
                    (Variables|Default|SetTB _array_element_3))
                  (bind _aspanel_widget_2 (Utilities|Casting|CastToPanelWidget _array_element_3)
                    (:then
                      (Utilities|Array|AppendArray (Variables|Default|GetNext) (Class|PanelWidget|GetAllChildren _aspanel_widget_2)))
                    (:CastFailed
                      (bind _asuser_widget_2 (Utilities|Casting|CastToUserWidget _array_element_3))
                      (bind _returnvalue_6 (Class|NaviUi|FindDecendentsOfClasses _asuser_widget_2 (Utilities|Array|MakeArray "/Script/UMG.CanvasPanel" "/Script/UMG.Overlay" "/Script/UMG.HorizontalBox" "/Script/UMG.VerticalBox" "/Script/UMG.GridPanel" "/Script/UMG.UniformGridPanel" "/Script/UMG.WrapBox" "/Script/UMG.ScrollBox" "/Script/UMG.SizeBox" "/Script/UMG.Border" "/Script/UMG.ScaleBox" "/Script/UMG.SafeZone" "/Script/UMG.NamedSlot" "/Script/UMG.WidgetSwitcher" "/Script/UMG.InvalidationBox" "/Script/UMG.RetainerBox" "/Script/UMG.StackBox" "/Script/UMG.BackgroundBlur") false))
                      (Utilities|Array|AppendArray (Variables|Default|GetNext) _returnvalue_6))))
                (Variables|Default|SetLevel (Variables|Default|GetNext))
                (if (and (not (Utilities|IsValid (Variables|Default|GetTB))) (> (Utilities|Array|Length (Variables|Default|GetLevel)) 0))
                  (Utilities|Array|Clear (Variables|Default|GetNext))
                  (for _array_element_4 (Variables|Default|GetLevel)
                    (if (and (Utilities|Enum|Equal(Enum) (Utilities|GetClassDisplayName (Utilities|GetClass _array_element_4)) "BottomToolbar_C") (not (Utilities|IsValid (Variables|Default|GetTB))))
                      (Variables|Default|SetTB _array_element_4))
                    (bind _aspanel_widget_3 (Utilities|Casting|CastToPanelWidget _array_element_4)
                      (:then
                        (Utilities|Array|AppendArray (Variables|Default|GetNext) (Class|PanelWidget|GetAllChildren _aspanel_widget_3)))
                      (:CastFailed
                        (bind _asuser_widget_3 (Utilities|Casting|CastToUserWidget _array_element_4))
                        (bind _returnvalue_7 (Class|NaviUi|FindDecendentsOfClasses _asuser_widget_3 (Utilities|Array|MakeArray "/Script/UMG.CanvasPanel" "/Script/UMG.Overlay" "/Script/UMG.HorizontalBox" "/Script/UMG.VerticalBox" "/Script/UMG.GridPanel" "/Script/UMG.UniformGridPanel" "/Script/UMG.WrapBox" "/Script/UMG.ScrollBox" "/Script/UMG.SizeBox" "/Script/UMG.Border" "/Script/UMG.ScaleBox" "/Script/UMG.SafeZone" "/Script/UMG.NamedSlot" "/Script/UMG.WidgetSwitcher" "/Script/UMG.InvalidationBox" "/Script/UMG.RetainerBox" "/Script/UMG.StackBox" "/Script/UMG.BackgroundBlur") false))
                        (Utilities|Array|AppendArray (Variables|Default|GetNext) _returnvalue_7))))
                  (Variables|Default|SetLevel (Variables|Default|GetNext))
                  (if (and (not (Utilities|IsValid (Variables|Default|GetTB))) (> (Utilities|Array|Length (Variables|Default|GetLevel)) 0))
                    (Utilities|Array|Clear (Variables|Default|GetNext))
                    (for _array_element_5 (Variables|Default|GetLevel)
                      (if (and (Utilities|Enum|Equal(Enum) (Utilities|GetClassDisplayName (Utilities|GetClass _array_element_5)) "BottomToolbar_C") (not (Utilities|IsValid (Variables|Default|GetTB))))
                        (Variables|Default|SetTB _array_element_5))
                      (bind _aspanel_widget_4 (Utilities|Casting|CastToPanelWidget _array_element_5)
                        (:then
                          (Utilities|Array|AppendArray (Variables|Default|GetNext) (Class|PanelWidget|GetAllChildren _aspanel_widget_4)))
                        (:CastFailed
                          (bind _asuser_widget_4 (Utilities|Casting|CastToUserWidget _array_element_5))
                          (bind _returnvalue_8 (Class|NaviUi|FindDecendentsOfClasses _asuser_widget_4 (Utilities|Array|MakeArray "/Script/UMG.CanvasPanel" "/Script/UMG.Overlay" "/Script/UMG.HorizontalBox" "/Script/UMG.VerticalBox" "/Script/UMG.GridPanel" "/Script/UMG.UniformGridPanel" "/Script/UMG.WrapBox" "/Script/UMG.ScrollBox" "/Script/UMG.SizeBox" "/Script/UMG.Border" "/Script/UMG.ScaleBox" "/Script/UMG.SafeZone" "/Script/UMG.NamedSlot" "/Script/UMG.WidgetSwitcher" "/Script/UMG.InvalidationBox" "/Script/UMG.RetainerBox" "/Script/UMG.StackBox" "/Script/UMG.BackgroundBlur") false))
                          (Utilities|Array|AppendArray (Variables|Default|GetNext) _returnvalue_8))))
                    (Variables|Default|SetLevel (Variables|Default|GetNext))))))
            (if (and (Utilities|IsValid (Variables|Default|GetTB)) (Widget|IsVisible (Variables|Default|GetTB)))
              (if (Utilities|IsValid (Widget|GetParent (Variables|Default|GetTB)))
                (Widget|Panel|AddChild (Widget|GetParent (Variables|Default|GetTB)) (Variables|Default|GetButton))
                (if (and (Utilities|IsValid (Class|WidgetLayoutLibrary|SlotasCanvasSlot (Variables|Default|GetTB))) (Utilities|IsValid (Class|WidgetLayoutLibrary|SlotasCanvasSlot (Variables|Default|GetButton))))
                  (Class|CanvasPanelSlot|SetAnchors (Class|WidgetLayoutLibrary|SlotasCanvasSlot (Variables|Default|GetButton)) "(Minimum=(X=0.500000,Y=1.000000),Maximum=(X=0.500000,Y=1.000000))")
                  (Class|CanvasPanelSlot|SetAlignment (Class|WidgetLayoutLibrary|SlotasCanvasSlot (Variables|Default|GetButton)) "(X=0.500000,Y=1.000000)")
                  (Class|CanvasPanelSlot|SetPosition (Class|WidgetLayoutLibrary|SlotasCanvasSlot (Variables|Default|GetButton)) (Math|Vector2D|MakeVector2D 0.0 (- 0.0 (+ (Math|Float|SelectFloat (.Y (Math|Vector2D|BreakVector2D (Class|Widget|GetDesiredSize (Variables|Default|GetTB)))) 1e+02 (and (> (.Y (Math|Vector2D|BreakVector2D (Class|Widget|GetDesiredSize (Variables|Default|GetTB)))) 1.0) (< (.Y (Math|Vector2D|BreakVector2D (Class|Widget|GetDesiredSize (Variables|Default|GetTB)))) 3e+02))) 3e+02))))
                  (Class|CanvasPanelSlot|SetAutoSize (Class|WidgetLayoutLibrary|SlotasCanvasSlot (Variables|Default|GetButton)) true)
                  (Variables|Default|SetPlaced true :!label _label)
                  (if (Variables|Default|GetDebug)
                    (Class|ModAPI|LogMessage (Class|ModAPI|GetModAPI) (Utilities|String|Append (Utilities|String|Append (Utilities|String|Append (Utilities|String|Append (Utilities|String|Append (Utilities|String|Append (Utilities|String|Append (Utilities|String|Append (Utilities|String|Append (Utilities|String|Append (Utilities|String|Append (Utilities|String|Append (Utilities|String|Append (Utilities|String|Append "RemakeMap: button placed above toolbar " "") (Utilities|GetDisplayName (Variables|Default|GetTB))) " (") (Utilities|GetClassDisplayName (Utilities|GetClass (Variables|Default|GetTB)))) ") in ") (Utilities|GetDisplayName (Widget|GetParent (Variables|Default|GetTB)))) " (") (Utilities|GetClassDisplayName (Utilities|GetClass (Widget|GetParent (Variables|Default|GetTB))))) "), canvas=") (Utilities|String|ToString(Boolean) (Utilities|IsValid (Class|WidgetLayoutLibrary|SlotasCanvasSlot (Variables|Default|GetTB))))) ", bar ") (Utilities|String|ToString(Vector2d) (Class|Widget|GetDesiredSize (Variables|Default|GetTB)))) ", try ") (Utilities|String|ToString(Integer) (Variables|Default|GetHudTries))) true))
                  (elif (Utilities|IsValid (Class|WidgetLayoutLibrary|SlotasOverlaySlot (Variables|Default|GetButton)))
                    (Layout|GridSlot|SetHorizontalAlignment (Class|WidgetLayoutLibrary|SlotasOverlaySlot (Variables|Default|GetButton)) "HAlign_Center")
                    (Layout|GridSlot|SetVerticalAlignment (Class|WidgetLayoutLibrary|SlotasOverlaySlot (Variables|Default|GetButton)) "VAlign_Bottom")
                    (Layout|BorderSlot|SetPadding (Class|WidgetLayoutLibrary|SlotasOverlaySlot (Variables|Default|GetButton)) (Utilities|Struct|MakeMargin (+ (.Y (Math|Vector2D|BreakVector2D (Class|Widget|GetDesiredSize (Variables|Default|GetTB)))) 2e+02)) :!class /Script/UMG.OverlaySlot)
                    (goto _label)
                    (else
                      (Widget|RemovefromParent (Variables|Default|GetButton))
                      (if (Variables|Default|GetDebug)
                        (Class|ModAPI|LogMessage (Class|ModAPI|GetModAPI) (Utilities|String|Append (Utilities|String|Append (Utilities|String|Append (Utilities|String|Append (Utilities|String|Append "RemakeMap: toolbar parent " "") (Utilities|GetDisplayName (Widget|GetParent (Variables|Default|GetTB)))) " (") (Utilities|GetClassDisplayName (Utilities|GetClass (Widget|GetParent (Variables|Default|GetTB))))) ") is not a canvas/overlay, button not shown") true))
                      (Variables|Default|SetPlaced true))))
                (else
                  (if (Variables|Default|GetDebug) :!label _label_2
                    (Class|ModAPI|LogMessage (Class|ModAPI|GetModAPI) (Utilities|String|Append (Utilities|String|Append (Utilities|String|Append (Utilities|String|Append (Utilities|String|Append (Utilities|String|Append "RemakeMap: toolbar not ready, try " "") (Utilities|String|ToString(Integer) (Variables|Default|GetHudTries))) ": HUDs=") (Utilities|String|ToString(Integer) (Utilities|Array|Length _foundwidgets))) " found=") (Utilities|String|ToString(Boolean) (Utilities|IsValid (Variables|Default|GetTB)))) true))
                  (if (< (Variables|Default|GetHudTries) 60)
                    (Variables|Default|SetHudTries (+ (Variables|Default|GetHudTries) 1))
                    (Utilities|Time|SetTimerbyFunctionName self "OnPlaceButton" 1.0)
                    (elif (Variables|Default|GetDebug)
                      (Class|ModAPI|LogMessage (Class|ModAPI|GetModAPI) "RemakeMap: no toolbar found, button not shown" true)))))
              (else
                (goto _label_2)))
            (else
              (goto _label_2))))
        (elif (Variables|Default|GetDebug)
          (Class|ModAPI|LogMessage (Class|ModAPI|GetModAPI) "RemakeMap: no button (loaded save or not day 1)" true)))
      (elif (< (Variables|Default|GetSetupTries) 10)
        (Variables|Default|SetSetupTries (+ (Variables|Default|GetSetupTries) 1))
        (Utilities|Time|SetTimerbyFunctionName self "OnLoaded" 1.0)))))

(event Custom|OnPlaceButton
  (bind _button (Variables|Default|GetButton))
  (bind _button_2 (Variables|Default|GetButton))
  (bind _returnvalue (Class|WidgetLayoutLibrary|SlotasCanvasSlot _button))
  (bind _returnvalue_2 (Class|WidgetLayoutLibrary|SlotasOverlaySlot _button_2))
  (if (not (or (Variables|Default|GetPlaced) (not (Utilities|IsValid (Variables|Default|GetButton)))))
    (bind _foundwidgets (Widget|GetAllWidgetsOfClass self "/Script/ProjectArco.PlayHud"))
    (if (> (Utilities|Array|Length _foundwidgets) 0)
      (Variables|Default|SetHud 0)
      (for _array_element _foundwidgets
        (Variables|Default|SetHud _array_element))
      (if (Variables|Default|GetDebug)
        (Class|ModAPI|LogMessage (Class|ModAPI|GetModAPI) (Utilities|String|Append (Utilities|String|Append (Utilities|String|Append (Utilities|String|Append "RemakeMap: walking HUD " "") (Utilities|GetDisplayName (Variables|Default|GetHud))) ", try ") (Utilities|String|ToString(Integer) (Variables|Default|GetHudTries))) true))
      (Utilities|Array|Clear (Variables|Default|GetLevel))
      (Utilities|Array|Add (Variables|Default|GetLevel) (Variables|Default|GetHud))
      (Variables|Default|SetTB 0)
      (if (and (not (Utilities|IsValid (Variables|Default|GetTB))) (> (Utilities|Array|Length (Variables|Default|GetLevel)) 0))
        (Utilities|Array|Clear (Variables|Default|GetNext))
        (for _array_element_2 (Variables|Default|GetLevel)
          (if (and (Utilities|Enum|Equal(Enum) (Utilities|GetClassDisplayName (Utilities|GetClass _array_element_2)) "BottomToolbar_C") (not (Utilities|IsValid (Variables|Default|GetTB))))
            (Variables|Default|SetTB _array_element_2))
          (bind _aspanel_widget (Utilities|Casting|CastToPanelWidget _array_element_2)
            (:then
              (Utilities|Array|AppendArray (Variables|Default|GetNext) (Class|PanelWidget|GetAllChildren _aspanel_widget)))
            (:CastFailed
              (bind _asuser_widget (Utilities|Casting|CastToUserWidget _array_element_2))
              (bind _returnvalue_3 (Class|NaviUi|FindDecendentsOfClasses _asuser_widget (Utilities|Array|MakeArray "/Script/UMG.CanvasPanel" "/Script/UMG.Overlay" "/Script/UMG.HorizontalBox" "/Script/UMG.VerticalBox" "/Script/UMG.GridPanel" "/Script/UMG.UniformGridPanel" "/Script/UMG.WrapBox" "/Script/UMG.ScrollBox" "/Script/UMG.SizeBox" "/Script/UMG.Border" "/Script/UMG.ScaleBox" "/Script/UMG.SafeZone" "/Script/UMG.NamedSlot" "/Script/UMG.WidgetSwitcher" "/Script/UMG.InvalidationBox" "/Script/UMG.RetainerBox" "/Script/UMG.StackBox" "/Script/UMG.BackgroundBlur") false))
              (Utilities|Array|AppendArray (Variables|Default|GetNext) _returnvalue_3))))
        (Variables|Default|SetLevel (Variables|Default|GetNext))
        (if (and (not (Utilities|IsValid (Variables|Default|GetTB))) (> (Utilities|Array|Length (Variables|Default|GetLevel)) 0))
          (Utilities|Array|Clear (Variables|Default|GetNext))
          (for _array_element_3 (Variables|Default|GetLevel)
            (if (and (Utilities|Enum|Equal(Enum) (Utilities|GetClassDisplayName (Utilities|GetClass _array_element_3)) "BottomToolbar_C") (not (Utilities|IsValid (Variables|Default|GetTB))))
              (Variables|Default|SetTB _array_element_3))
            (bind _aspanel_widget_2 (Utilities|Casting|CastToPanelWidget _array_element_3)
              (:then
                (Utilities|Array|AppendArray (Variables|Default|GetNext) (Class|PanelWidget|GetAllChildren _aspanel_widget_2)))
              (:CastFailed
                (bind _asuser_widget_2 (Utilities|Casting|CastToUserWidget _array_element_3))
                (bind _returnvalue_4 (Class|NaviUi|FindDecendentsOfClasses _asuser_widget_2 (Utilities|Array|MakeArray "/Script/UMG.CanvasPanel" "/Script/UMG.Overlay" "/Script/UMG.HorizontalBox" "/Script/UMG.VerticalBox" "/Script/UMG.GridPanel" "/Script/UMG.UniformGridPanel" "/Script/UMG.WrapBox" "/Script/UMG.ScrollBox" "/Script/UMG.SizeBox" "/Script/UMG.Border" "/Script/UMG.ScaleBox" "/Script/UMG.SafeZone" "/Script/UMG.NamedSlot" "/Script/UMG.WidgetSwitcher" "/Script/UMG.InvalidationBox" "/Script/UMG.RetainerBox" "/Script/UMG.StackBox" "/Script/UMG.BackgroundBlur") false))
                (Utilities|Array|AppendArray (Variables|Default|GetNext) _returnvalue_4))))
          (Variables|Default|SetLevel (Variables|Default|GetNext))
          (if (and (not (Utilities|IsValid (Variables|Default|GetTB))) (> (Utilities|Array|Length (Variables|Default|GetLevel)) 0))
            (Utilities|Array|Clear (Variables|Default|GetNext))
            (for _array_element_4 (Variables|Default|GetLevel)
              (if (and (Utilities|Enum|Equal(Enum) (Utilities|GetClassDisplayName (Utilities|GetClass _array_element_4)) "BottomToolbar_C") (not (Utilities|IsValid (Variables|Default|GetTB))))
                (Variables|Default|SetTB _array_element_4))
              (bind _aspanel_widget_3 (Utilities|Casting|CastToPanelWidget _array_element_4)
                (:then
                  (Utilities|Array|AppendArray (Variables|Default|GetNext) (Class|PanelWidget|GetAllChildren _aspanel_widget_3)))
                (:CastFailed
                  (bind _asuser_widget_3 (Utilities|Casting|CastToUserWidget _array_element_4))
                  (bind _returnvalue_5 (Class|NaviUi|FindDecendentsOfClasses _asuser_widget_3 (Utilities|Array|MakeArray "/Script/UMG.CanvasPanel" "/Script/UMG.Overlay" "/Script/UMG.HorizontalBox" "/Script/UMG.VerticalBox" "/Script/UMG.GridPanel" "/Script/UMG.UniformGridPanel" "/Script/UMG.WrapBox" "/Script/UMG.ScrollBox" "/Script/UMG.SizeBox" "/Script/UMG.Border" "/Script/UMG.ScaleBox" "/Script/UMG.SafeZone" "/Script/UMG.NamedSlot" "/Script/UMG.WidgetSwitcher" "/Script/UMG.InvalidationBox" "/Script/UMG.RetainerBox" "/Script/UMG.StackBox" "/Script/UMG.BackgroundBlur") false))
                  (Utilities|Array|AppendArray (Variables|Default|GetNext) _returnvalue_5))))
            (Variables|Default|SetLevel (Variables|Default|GetNext))
            (if (and (not (Utilities|IsValid (Variables|Default|GetTB))) (> (Utilities|Array|Length (Variables|Default|GetLevel)) 0))
              (Utilities|Array|Clear (Variables|Default|GetNext))
              (for _array_element_5 (Variables|Default|GetLevel)
                (if (and (Utilities|Enum|Equal(Enum) (Utilities|GetClassDisplayName (Utilities|GetClass _array_element_5)) "BottomToolbar_C") (not (Utilities|IsValid (Variables|Default|GetTB))))
                  (Variables|Default|SetTB _array_element_5))
                (bind _aspanel_widget_4 (Utilities|Casting|CastToPanelWidget _array_element_5)
                  (:then
                    (Utilities|Array|AppendArray (Variables|Default|GetNext) (Class|PanelWidget|GetAllChildren _aspanel_widget_4)))
                  (:CastFailed
                    (bind _asuser_widget_4 (Utilities|Casting|CastToUserWidget _array_element_5))
                    (bind _returnvalue_6 (Class|NaviUi|FindDecendentsOfClasses _asuser_widget_4 (Utilities|Array|MakeArray "/Script/UMG.CanvasPanel" "/Script/UMG.Overlay" "/Script/UMG.HorizontalBox" "/Script/UMG.VerticalBox" "/Script/UMG.GridPanel" "/Script/UMG.UniformGridPanel" "/Script/UMG.WrapBox" "/Script/UMG.ScrollBox" "/Script/UMG.SizeBox" "/Script/UMG.Border" "/Script/UMG.ScaleBox" "/Script/UMG.SafeZone" "/Script/UMG.NamedSlot" "/Script/UMG.WidgetSwitcher" "/Script/UMG.InvalidationBox" "/Script/UMG.RetainerBox" "/Script/UMG.StackBox" "/Script/UMG.BackgroundBlur") false))
                    (Utilities|Array|AppendArray (Variables|Default|GetNext) _returnvalue_6))))
              (Variables|Default|SetLevel (Variables|Default|GetNext))))))
      (if (and (Utilities|IsValid (Variables|Default|GetTB)) (Widget|IsVisible (Variables|Default|GetTB)))
        (if (Utilities|IsValid (Widget|GetParent (Variables|Default|GetTB)))
          (Widget|Panel|AddChild (Widget|GetParent (Variables|Default|GetTB)) (Variables|Default|GetButton))
          (if (and (Utilities|IsValid (Class|WidgetLayoutLibrary|SlotasCanvasSlot (Variables|Default|GetTB))) (Utilities|IsValid _returnvalue))
            (Class|CanvasPanelSlot|SetAnchors _returnvalue "(Minimum=(X=0.500000,Y=1.000000),Maximum=(X=0.500000,Y=1.000000))")
            (Class|CanvasPanelSlot|SetAlignment _returnvalue "(X=0.500000,Y=1.000000)")
            (Class|CanvasPanelSlot|SetPosition _returnvalue (Math|Vector2D|MakeVector2D 0.0 (- 0.0 (+ (Math|Float|SelectFloat (.Y (Math|Vector2D|BreakVector2D (Class|Widget|GetDesiredSize (Variables|Default|GetTB)))) 1e+02 (and (> (.Y (Math|Vector2D|BreakVector2D (Class|Widget|GetDesiredSize (Variables|Default|GetTB)))) 1.0) (< (.Y (Math|Vector2D|BreakVector2D (Class|Widget|GetDesiredSize (Variables|Default|GetTB)))) 3e+02))) 3e+02))))
            (Class|CanvasPanelSlot|SetAutoSize _returnvalue true)
            (Variables|Default|SetPlaced true :!label _label)
            (if (Variables|Default|GetDebug)
              (Class|ModAPI|LogMessage (Class|ModAPI|GetModAPI) (Utilities|String|Append (Utilities|String|Append (Utilities|String|Append (Utilities|String|Append (Utilities|String|Append (Utilities|String|Append (Utilities|String|Append (Utilities|String|Append (Utilities|String|Append (Utilities|String|Append (Utilities|String|Append (Utilities|String|Append (Utilities|String|Append (Utilities|String|Append "RemakeMap: button placed above toolbar " "") (Utilities|GetDisplayName (Variables|Default|GetTB))) " (") (Utilities|GetClassDisplayName (Utilities|GetClass (Variables|Default|GetTB)))) ") in ") (Utilities|GetDisplayName (Widget|GetParent (Variables|Default|GetTB)))) " (") (Utilities|GetClassDisplayName (Utilities|GetClass (Widget|GetParent (Variables|Default|GetTB))))) "), canvas=") (Utilities|String|ToString(Boolean) (Utilities|IsValid (Class|WidgetLayoutLibrary|SlotasCanvasSlot (Variables|Default|GetTB))))) ", bar ") (Utilities|String|ToString(Vector2d) (Class|Widget|GetDesiredSize (Variables|Default|GetTB)))) ", try ") (Utilities|String|ToString(Integer) (Variables|Default|GetHudTries))) true))
            (elif (Utilities|IsValid _returnvalue_2)
              (Layout|GridSlot|SetHorizontalAlignment _returnvalue_2 "HAlign_Center")
              (Layout|GridSlot|SetVerticalAlignment _returnvalue_2 "VAlign_Bottom")
              (Layout|BorderSlot|SetPadding _returnvalue_2 (Utilities|Struct|MakeMargin (+ (.Y (Math|Vector2D|BreakVector2D (Class|Widget|GetDesiredSize (Variables|Default|GetTB)))) 2e+02)) :!class /Script/UMG.OverlaySlot)
              (goto _label)
              (else
                (Widget|RemovefromParent (Variables|Default|GetButton))
                (if (Variables|Default|GetDebug)
                  (Class|ModAPI|LogMessage (Class|ModAPI|GetModAPI) (Utilities|String|Append (Utilities|String|Append (Utilities|String|Append (Utilities|String|Append (Utilities|String|Append "RemakeMap: toolbar parent " "") (Utilities|GetDisplayName (Widget|GetParent (Variables|Default|GetTB)))) " (") (Utilities|GetClassDisplayName (Utilities|GetClass (Widget|GetParent (Variables|Default|GetTB))))) ") is not a canvas/overlay, button not shown") true))
                (Variables|Default|SetPlaced true))))
          (else
            (if (Variables|Default|GetDebug) :!label _label_2
              (Class|ModAPI|LogMessage (Class|ModAPI|GetModAPI) (Utilities|String|Append (Utilities|String|Append (Utilities|String|Append (Utilities|String|Append (Utilities|String|Append (Utilities|String|Append "RemakeMap: toolbar not ready, try " "") (Utilities|String|ToString(Integer) (Variables|Default|GetHudTries))) ": HUDs=") (Utilities|String|ToString(Integer) (Utilities|Array|Length _foundwidgets))) " found=") (Utilities|String|ToString(Boolean) (Utilities|IsValid (Variables|Default|GetTB)))) true))
            (if (< (Variables|Default|GetHudTries) 60)
              (Variables|Default|SetHudTries (+ (Variables|Default|GetHudTries) 1))
              (Utilities|Time|SetTimerbyFunctionName self "OnPlaceButton" 1.0)
              (elif (Variables|Default|GetDebug)
                (Class|ModAPI|LogMessage (Class|ModAPI|GetModAPI) "RemakeMap: no toolbar found, button not shown" true)))))
        (else
          (goto _label_2)))
      (else
        (goto _label_2)))))

(event Custom|OnRemakeClick
  (if (Variables|Default|GetArmed)
    (if (Variables|Default|GetDebug)
      (Class|ModAPI|LogMessage (Class|ModAPI|GetModAPI) "RemakeMap: second click, remaking" true))
    (Variables|Default|SetNewSeed (Math|Random|RandomIntegerinRange 1 9999999))
    (Variables|Default|SetNewRaw (Math|Random|RandomFloatinRange 0.0 1e+03))
    (Class|ArcoGameInstance|SetNewMapPreference self "Seed" (Utilities|String|StringToName (Utilities|String|ToString(Integer) (Variables|Default|GetNewSeed))) (Variables|Default|GetNewRaw))
    (if (Variables|Default|GetDebug)
      (Class|ModAPI|LogMessage (Class|ModAPI|GetModAPI) (Utilities|String|Append (Utilities|String|Append (Utilities|String|Append (Utilities|String|Append (Utilities|String|Append "RemakeMap: new seed " "") (Utilities|String|ToString(Integer) (Variables|Default|GetNewSeed))) " (raw ") (Utilities|String|ToString(Float) (Variables|Default|GetNewRaw))) ")") true))
    (Class|ArcoGameInstance|EnterPlay self "" "NEW_GENERATION" "SAVED_GAMES" false)
    (if (Variables|Default|GetDebug)
      (Class|ModAPI|LogMessage (Class|ModAPI|GetModAPI) "RemakeMap: EnterPlay(NEW_GENERATION) called" true))
    (else
      (Variables|Default|SetArmed true)
      (Rendering|Components|TextRender|SetText (Variables|/Game/Mods/RemakeMap/WBP_RemakeButton.WBP_RemakeButton_C|GetLabel (Variables|Default|GetButton)) (Utilities|Text|ToText(String) "Click again to remake the map"))
      (if (Variables|Default|GetDebug)
        (Class|ModAPI|LogMessage (Class|ModAPI|GetModAPI) "RemakeMap: armed (first click)" true)))))

(event EventBeginPlay
  (bind _returnvalue (Class|ModAPI|GetModAPI))
  (EventDispatchers|BindEventtoOnLoadingFinished _returnvalue (delegate Custom|OnLoaded))
  (EventDispatchers|BindEventtoOnDayStart _returnvalue (delegate Custom|OnDayStart))
  (if (not (Variables|Default|GetReady))
    (if (Utilities|IsValid (Game|GetPlayerController 0))
      (Variables|Default|SetReady true)
      (bind _returnvalue_2 (Class|ModAPI|ReadModTextFile (Class|ModAPI|GetModAPI) "RemakeMapConfig" "debug"))
      (Variables|Default|SetDebug (not (Utilities|Array|IsEmpty _returnvalue_2)))
      (if (Variables|Default|GetDebug)
        (Class|ModAPI|LogMessage (Class|ModAPI|GetModAPI) "RemakeMap ready (v17)" true))
      (bind (_out_isvalid _returnvalue_3) (Class|ArcoSystems|GetArcoSys))
      (Variables|Default|SetArco _returnvalue_3)
      (bind _returnvalue_4 (Class|ArcoSystems|IsSaveGame (Variables|Default|GetArco)))
      (if (Variables|Default|GetDebug)
        (Class|ModAPI|LogMessage (Class|ModAPI|GetModAPI) (Utilities|String|Append (Utilities|String|Append (Utilities|String|Append (Utilities|String|Append (Utilities|String|Append (Utilities|String|Append (Utilities|String|Append (Utilities|String|Append (Utilities|String|Append (Utilities|String|Append "RemakeMap: arco valid=" "") (Utilities|String|ToString(Boolean) _out_isvalid)) " save game=") (Utilities|String|ToString(Boolean) _returnvalue_4)) " day=") (Utilities|String|ToString(Integer) (Variables|/Script/ProjectArco.WorldTime|Getm_day (Variables|/Script/ProjectArco.ArcoSystems|Getm_worldTime (Variables|Default|GetArco))))) " colony=") (Class|ArcoSystems|GetColonyName (Variables|Default|GetArco))) " debt=") (Utilities|String|ToString(Float) (Class|ArcoSystems|GetDebtMultiplier (Variables|Default|GetArco)))) true))
      (if (and (not _returnvalue_4) (<= (Variables|/Script/ProjectArco.WorldTime|Getm_day (Variables|/Script/ProjectArco.ArcoSystems|Getm_worldTime (Variables|Default|GetArco))) 1))
        (bind _returnvalue_5 (UserInterface|CreateWidget "/Game/Mods/RemakeMap/WBP_RemakeButton.WBP_RemakeButton_C" (Game|GetPlayerController 0)))
        (Variables|Default|SetButton _returnvalue_5)
        (Rendering|Components|TextRender|SetText (Variables|/Game/Mods/RemakeMap/WBP_RemakeButton.WBP_RemakeButton_C|GetLabel (Variables|Default|GetButton)) (Utilities|Text|ToText(String) "Remake map"))
        (EventDispatchers|BindEventtoOnClicked (Variables|/Game/Mods/RemakeMap/WBP_RemakeButton.WBP_RemakeButton_C|GetBtn (Variables|Default|GetButton)) (delegate Custom|OnRemakeClick))
        (if (not (or (Variables|Default|GetPlaced) (not (Utilities|IsValid (Variables|Default|GetButton)))))
          (bind _foundwidgets (Widget|GetAllWidgetsOfClass self "/Script/ProjectArco.PlayHud"))
          (if (> (Utilities|Array|Length _foundwidgets) 0)
            (Variables|Default|SetHud 0)
            (for _array_element _foundwidgets
              (Variables|Default|SetHud _array_element))
            (if (Variables|Default|GetDebug)
              (Class|ModAPI|LogMessage (Class|ModAPI|GetModAPI) (Utilities|String|Append (Utilities|String|Append (Utilities|String|Append (Utilities|String|Append "RemakeMap: walking HUD " "") (Utilities|GetDisplayName (Variables|Default|GetHud))) ", try ") (Utilities|String|ToString(Integer) (Variables|Default|GetHudTries))) true))
            (Utilities|Array|Clear (Variables|Default|GetLevel))
            (Utilities|Array|Add (Variables|Default|GetLevel) (Variables|Default|GetHud))
            (Variables|Default|SetTB 0)
            (if (and (not (Utilities|IsValid (Variables|Default|GetTB))) (> (Utilities|Array|Length (Variables|Default|GetLevel)) 0))
              (Utilities|Array|Clear (Variables|Default|GetNext))
              (for _array_element_2 (Variables|Default|GetLevel)
                (if (and (Utilities|Enum|Equal(Enum) (Utilities|GetClassDisplayName (Utilities|GetClass _array_element_2)) "BottomToolbar_C") (not (Utilities|IsValid (Variables|Default|GetTB))))
                  (Variables|Default|SetTB _array_element_2))
                (bind _aspanel_widget (Utilities|Casting|CastToPanelWidget _array_element_2)
                  (:then
                    (Utilities|Array|AppendArray (Variables|Default|GetNext) (Class|PanelWidget|GetAllChildren _aspanel_widget)))
                  (:CastFailed
                    (bind _asuser_widget (Utilities|Casting|CastToUserWidget _array_element_2))
                    (bind _returnvalue_6 (Class|NaviUi|FindDecendentsOfClasses _asuser_widget (Utilities|Array|MakeArray "/Script/UMG.CanvasPanel" "/Script/UMG.Overlay" "/Script/UMG.HorizontalBox" "/Script/UMG.VerticalBox" "/Script/UMG.GridPanel" "/Script/UMG.UniformGridPanel" "/Script/UMG.WrapBox" "/Script/UMG.ScrollBox" "/Script/UMG.SizeBox" "/Script/UMG.Border" "/Script/UMG.ScaleBox" "/Script/UMG.SafeZone" "/Script/UMG.NamedSlot" "/Script/UMG.WidgetSwitcher" "/Script/UMG.InvalidationBox" "/Script/UMG.RetainerBox" "/Script/UMG.StackBox" "/Script/UMG.BackgroundBlur") false))
                    (Utilities|Array|AppendArray (Variables|Default|GetNext) _returnvalue_6))))
              (Variables|Default|SetLevel (Variables|Default|GetNext))
              (if (and (not (Utilities|IsValid (Variables|Default|GetTB))) (> (Utilities|Array|Length (Variables|Default|GetLevel)) 0))
                (Utilities|Array|Clear (Variables|Default|GetNext))
                (for _array_element_3 (Variables|Default|GetLevel)
                  (if (and (Utilities|Enum|Equal(Enum) (Utilities|GetClassDisplayName (Utilities|GetClass _array_element_3)) "BottomToolbar_C") (not (Utilities|IsValid (Variables|Default|GetTB))))
                    (Variables|Default|SetTB _array_element_3))
                  (bind _aspanel_widget_2 (Utilities|Casting|CastToPanelWidget _array_element_3)
                    (:then
                      (Utilities|Array|AppendArray (Variables|Default|GetNext) (Class|PanelWidget|GetAllChildren _aspanel_widget_2)))
                    (:CastFailed
                      (bind _asuser_widget_2 (Utilities|Casting|CastToUserWidget _array_element_3))
                      (bind _returnvalue_7 (Class|NaviUi|FindDecendentsOfClasses _asuser_widget_2 (Utilities|Array|MakeArray "/Script/UMG.CanvasPanel" "/Script/UMG.Overlay" "/Script/UMG.HorizontalBox" "/Script/UMG.VerticalBox" "/Script/UMG.GridPanel" "/Script/UMG.UniformGridPanel" "/Script/UMG.WrapBox" "/Script/UMG.ScrollBox" "/Script/UMG.SizeBox" "/Script/UMG.Border" "/Script/UMG.ScaleBox" "/Script/UMG.SafeZone" "/Script/UMG.NamedSlot" "/Script/UMG.WidgetSwitcher" "/Script/UMG.InvalidationBox" "/Script/UMG.RetainerBox" "/Script/UMG.StackBox" "/Script/UMG.BackgroundBlur") false))
                      (Utilities|Array|AppendArray (Variables|Default|GetNext) _returnvalue_7))))
                (Variables|Default|SetLevel (Variables|Default|GetNext))
                (if (and (not (Utilities|IsValid (Variables|Default|GetTB))) (> (Utilities|Array|Length (Variables|Default|GetLevel)) 0))
                  (Utilities|Array|Clear (Variables|Default|GetNext))
                  (for _array_element_4 (Variables|Default|GetLevel)
                    (if (and (Utilities|Enum|Equal(Enum) (Utilities|GetClassDisplayName (Utilities|GetClass _array_element_4)) "BottomToolbar_C") (not (Utilities|IsValid (Variables|Default|GetTB))))
                      (Variables|Default|SetTB _array_element_4))
                    (bind _aspanel_widget_3 (Utilities|Casting|CastToPanelWidget _array_element_4)
                      (:then
                        (Utilities|Array|AppendArray (Variables|Default|GetNext) (Class|PanelWidget|GetAllChildren _aspanel_widget_3)))
                      (:CastFailed
                        (bind _asuser_widget_3 (Utilities|Casting|CastToUserWidget _array_element_4))
                        (bind _returnvalue_8 (Class|NaviUi|FindDecendentsOfClasses _asuser_widget_3 (Utilities|Array|MakeArray "/Script/UMG.CanvasPanel" "/Script/UMG.Overlay" "/Script/UMG.HorizontalBox" "/Script/UMG.VerticalBox" "/Script/UMG.GridPanel" "/Script/UMG.UniformGridPanel" "/Script/UMG.WrapBox" "/Script/UMG.ScrollBox" "/Script/UMG.SizeBox" "/Script/UMG.Border" "/Script/UMG.ScaleBox" "/Script/UMG.SafeZone" "/Script/UMG.NamedSlot" "/Script/UMG.WidgetSwitcher" "/Script/UMG.InvalidationBox" "/Script/UMG.RetainerBox" "/Script/UMG.StackBox" "/Script/UMG.BackgroundBlur") false))
                        (Utilities|Array|AppendArray (Variables|Default|GetNext) _returnvalue_8))))
                  (Variables|Default|SetLevel (Variables|Default|GetNext))
                  (if (and (not (Utilities|IsValid (Variables|Default|GetTB))) (> (Utilities|Array|Length (Variables|Default|GetLevel)) 0))
                    (Utilities|Array|Clear (Variables|Default|GetNext))
                    (for _array_element_5 (Variables|Default|GetLevel)
                      (if (and (Utilities|Enum|Equal(Enum) (Utilities|GetClassDisplayName (Utilities|GetClass _array_element_5)) "BottomToolbar_C") (not (Utilities|IsValid (Variables|Default|GetTB))))
                        (Variables|Default|SetTB _array_element_5))
                      (bind _aspanel_widget_4 (Utilities|Casting|CastToPanelWidget _array_element_5)
                        (:then
                          (Utilities|Array|AppendArray (Variables|Default|GetNext) (Class|PanelWidget|GetAllChildren _aspanel_widget_4)))
                        (:CastFailed
                          (bind _asuser_widget_4 (Utilities|Casting|CastToUserWidget _array_element_5))
                          (bind _returnvalue_9 (Class|NaviUi|FindDecendentsOfClasses _asuser_widget_4 (Utilities|Array|MakeArray "/Script/UMG.CanvasPanel" "/Script/UMG.Overlay" "/Script/UMG.HorizontalBox" "/Script/UMG.VerticalBox" "/Script/UMG.GridPanel" "/Script/UMG.UniformGridPanel" "/Script/UMG.WrapBox" "/Script/UMG.ScrollBox" "/Script/UMG.SizeBox" "/Script/UMG.Border" "/Script/UMG.ScaleBox" "/Script/UMG.SafeZone" "/Script/UMG.NamedSlot" "/Script/UMG.WidgetSwitcher" "/Script/UMG.InvalidationBox" "/Script/UMG.RetainerBox" "/Script/UMG.StackBox" "/Script/UMG.BackgroundBlur") false))
                          (Utilities|Array|AppendArray (Variables|Default|GetNext) _returnvalue_9))))
                    (Variables|Default|SetLevel (Variables|Default|GetNext))))))
            (if (and (Utilities|IsValid (Variables|Default|GetTB)) (Widget|IsVisible (Variables|Default|GetTB)))
              (if (Utilities|IsValid (Widget|GetParent (Variables|Default|GetTB)))
                (Widget|Panel|AddChild (Widget|GetParent (Variables|Default|GetTB)) (Variables|Default|GetButton))
                (if (and (Utilities|IsValid (Class|WidgetLayoutLibrary|SlotasCanvasSlot (Variables|Default|GetTB))) (Utilities|IsValid (Class|WidgetLayoutLibrary|SlotasCanvasSlot (Variables|Default|GetButton))))
                  (Class|CanvasPanelSlot|SetAnchors (Class|WidgetLayoutLibrary|SlotasCanvasSlot (Variables|Default|GetButton)) "(Minimum=(X=0.500000,Y=1.000000),Maximum=(X=0.500000,Y=1.000000))")
                  (Class|CanvasPanelSlot|SetAlignment (Class|WidgetLayoutLibrary|SlotasCanvasSlot (Variables|Default|GetButton)) "(X=0.500000,Y=1.000000)")
                  (Class|CanvasPanelSlot|SetPosition (Class|WidgetLayoutLibrary|SlotasCanvasSlot (Variables|Default|GetButton)) (Math|Vector2D|MakeVector2D 0.0 (- 0.0 (+ (Math|Float|SelectFloat (.Y (Math|Vector2D|BreakVector2D (Class|Widget|GetDesiredSize (Variables|Default|GetTB)))) 1e+02 (and (> (.Y (Math|Vector2D|BreakVector2D (Class|Widget|GetDesiredSize (Variables|Default|GetTB)))) 1.0) (< (.Y (Math|Vector2D|BreakVector2D (Class|Widget|GetDesiredSize (Variables|Default|GetTB)))) 3e+02))) 3e+02))))
                  (Class|CanvasPanelSlot|SetAutoSize (Class|WidgetLayoutLibrary|SlotasCanvasSlot (Variables|Default|GetButton)) true)
                  (Variables|Default|SetPlaced true :!label _label)
                  (if (Variables|Default|GetDebug)
                    (Class|ModAPI|LogMessage (Class|ModAPI|GetModAPI) (Utilities|String|Append (Utilities|String|Append (Utilities|String|Append (Utilities|String|Append (Utilities|String|Append (Utilities|String|Append (Utilities|String|Append (Utilities|String|Append (Utilities|String|Append (Utilities|String|Append (Utilities|String|Append (Utilities|String|Append (Utilities|String|Append (Utilities|String|Append "RemakeMap: button placed above toolbar " "") (Utilities|GetDisplayName (Variables|Default|GetTB))) " (") (Utilities|GetClassDisplayName (Utilities|GetClass (Variables|Default|GetTB)))) ") in ") (Utilities|GetDisplayName (Widget|GetParent (Variables|Default|GetTB)))) " (") (Utilities|GetClassDisplayName (Utilities|GetClass (Widget|GetParent (Variables|Default|GetTB))))) "), canvas=") (Utilities|String|ToString(Boolean) (Utilities|IsValid (Class|WidgetLayoutLibrary|SlotasCanvasSlot (Variables|Default|GetTB))))) ", bar ") (Utilities|String|ToString(Vector2d) (Class|Widget|GetDesiredSize (Variables|Default|GetTB)))) ", try ") (Utilities|String|ToString(Integer) (Variables|Default|GetHudTries))) true))
                  (elif (Utilities|IsValid (Class|WidgetLayoutLibrary|SlotasOverlaySlot (Variables|Default|GetButton)))
                    (Layout|GridSlot|SetHorizontalAlignment (Class|WidgetLayoutLibrary|SlotasOverlaySlot (Variables|Default|GetButton)) "HAlign_Center")
                    (Layout|GridSlot|SetVerticalAlignment (Class|WidgetLayoutLibrary|SlotasOverlaySlot (Variables|Default|GetButton)) "VAlign_Bottom")
                    (Layout|BorderSlot|SetPadding (Class|WidgetLayoutLibrary|SlotasOverlaySlot (Variables|Default|GetButton)) (Utilities|Struct|MakeMargin (+ (.Y (Math|Vector2D|BreakVector2D (Class|Widget|GetDesiredSize (Variables|Default|GetTB)))) 2e+02)) :!class /Script/UMG.OverlaySlot)
                    (goto _label)
                    (else
                      (Widget|RemovefromParent (Variables|Default|GetButton))
                      (if (Variables|Default|GetDebug)
                        (Class|ModAPI|LogMessage (Class|ModAPI|GetModAPI) (Utilities|String|Append (Utilities|String|Append (Utilities|String|Append (Utilities|String|Append (Utilities|String|Append "RemakeMap: toolbar parent " "") (Utilities|GetDisplayName (Widget|GetParent (Variables|Default|GetTB)))) " (") (Utilities|GetClassDisplayName (Utilities|GetClass (Widget|GetParent (Variables|Default|GetTB))))) ") is not a canvas/overlay, button not shown") true))
                      (Variables|Default|SetPlaced true))))
                (else
                  (if (Variables|Default|GetDebug) :!label _label_2
                    (Class|ModAPI|LogMessage (Class|ModAPI|GetModAPI) (Utilities|String|Append (Utilities|String|Append (Utilities|String|Append (Utilities|String|Append (Utilities|String|Append (Utilities|String|Append "RemakeMap: toolbar not ready, try " "") (Utilities|String|ToString(Integer) (Variables|Default|GetHudTries))) ": HUDs=") (Utilities|String|ToString(Integer) (Utilities|Array|Length _foundwidgets))) " found=") (Utilities|String|ToString(Boolean) (Utilities|IsValid (Variables|Default|GetTB)))) true))
                  (if (< (Variables|Default|GetHudTries) 60)
                    (Variables|Default|SetHudTries (+ (Variables|Default|GetHudTries) 1))
                    (Utilities|Time|SetTimerbyFunctionName self "OnPlaceButton" 1.0)
                    (elif (Variables|Default|GetDebug)
                      (Class|ModAPI|LogMessage (Class|ModAPI|GetModAPI) "RemakeMap: no toolbar found, button not shown" true)))))
              (else
                (goto _label_2)))
            (else
              (goto _label_2))))
        (elif (Variables|Default|GetDebug)
          (Class|ModAPI|LogMessage (Class|ModAPI|GetModAPI) "RemakeMap: no button (loaded save or not day 1)" true)))
      (elif (< (Variables|Default|GetSetupTries) 10)
        (Variables|Default|SetSetupTries (+ (Variables|Default|GetSetupTries) 1))
        (Utilities|Time|SetTimerbyFunctionName self "OnLoaded" 1.0)))))

(fn ConstructionScript)